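; Player car vehicle pawn that drives through VehicleMovement, creates the HUD on BeginPlay and opens a pause menu on P.
; A child-actor turret snaps to the mesh's "turret" socket, rotates from stick axes past a deadzone, and fires while decrementing Ammo.
; H and J directly drain Health and Energy, apparently for testing.
; Handbrake press and release both set the handbrake to false, so it never engages.
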(event EventBeginPlay
  ;[1 1 1] HUD
  (bind _returnvalue (UserInterface|CreateWidget "/Game/UI/UMG/HUD.HUD_C"))
  (bind _output_get (Variables|Default|SetplayerHUD _returnvalue))
  (UserInterface|Viewport|AddtoViewport _output_get 0)
  (Input|SetInputModeGameOnly (Game|GetPlayerController 0)))

(event Collision|EventActorBeginOverlap
  (params (OtherActor :type Actor%20Object%20Reference)))

(event Input|ActionEvents|InputActionHandbrake
  (params (Key :type Key%20Structure))
  (bind _vehiclemovement (Variables|Default|GetVehicleMovement))
  ;[1 1 1] playerMovement
  (:Pressed
    (Class|WheeledVehicleMovementComponent|SetHandbrakeInput _vehiclemovement false))
  (:Released
    (Class|WheeledVehicleMovementComponent|SetHandbrakeInput _vehiclemovement false)))

(event Input|ActionEvents|InputActionfire
  (params (Key :type Key%20Structure))
  ;[1 1 1] Controls and inputs
  (:Pressed
    (bind _ascar_turret (Utilities|Casting|CastTocarTurret (Variables|/Script/Engine.ChildActorComponent|GetChildActor (Variables|Default|GetcarWeapon))))
    (Default|FireWeapon _ascar_turret)
    (Math|Integer|DecrementInt (Variables|Default|Getammo))))

(event Input|AxisEvents|InputAxisForeward
  (params (AxisValue :type Float%20%28single-precision%29))
  ;[1 1 1] playerMovement
  (Class|WheeledVehicleMovementComponent|SetThrottleInput (Variables|Default|GetVehicleMovement) AxisValue))

(event Input|AxisEvents|InputAxisRight
  (params (AxisValue :type Float%20%28single-precision%29))
  ;[1 1 1] playerMovement
  (Class|WheeledVehicleMovementComponent|SetSteeringInput (Variables|Default|GetVehicleMovement) AxisValue))

(event Input|AxisEvents|InputAxisturretRotateRight
  (params (AxisValue :type Float%20%28single-precision%29))
  (if (> (Math|Vector|VectorLength (Math|Vector|MakeVector (stale Input|AxisEvents|InputAxisturretRotateUp AxisValue) AxisValue 0.0)) 0.25)
    (Transformation|SetRelativeRotation (Variables|Default|GetcarWeapon) (Math|Conversions|RotationFromXVector (Math|Vector|MakeVector (stale Input|AxisEvents|InputAxisturretRotateUp AxisValue) AxisValue 0.0)) false false)))

(event Input|AxisEvents|InputAxisturretRotateUp
  (params (AxisValue :type Float%20%28single-precision%29))
  (if (> (Math|Vector|VectorLength (Math|Vector|MakeVector AxisValue (stale Input|AxisEvents|InputAxisturretRotateRight AxisValue) 0.0)) 0.25)
    (Transformation|SetRelativeRotation (Variables|Default|GetcarWeapon) (Math|Conversions|RotationFromXVector (Math|Vector|MakeVector AxisValue (stale Input|AxisEvents|InputAxisturretRotateRight AxisValue) 0.0)) false false)))

(event Input|KeyboardEvents|H
  (params (Key :type Key%20Structure))
  ;[1 1 1] Controls and inputs
  (:Pressed
    (Variables|Default|Sethealth (- (Variables|Default|Gethealth) 0.25))))

(event Input|KeyboardEvents|J
  (params (Key :type Key%20Structure))
  ;[1 1 1] Controls and inputs
  (:Pressed
    (Variables|Default|Setenergy (- (Variables|Default|Getenergy) 1.0))))

(event Input|KeyboardEvents|P
  (params (Key :type Key%20Structure))
  ;[1 1 1] Controls and inputs
  (:Pressed
    (Utilities|IsValid (Variables|Default|GetpauseMenu)
      (:Is%20Valid
        _)
      (:Is%20Not%20Valid
        (bind _returnvalue (UserInterface|CreateWidget "/Game/UI/UMG/PauseMenu.PauseMenu_C"))
        (Variables|Default|SetpauseMenu _returnvalue)))
    (Input|SetInputModeUIOnly (Game|GetPlayerController 0) (Variables|Default|GetpauseMenu) "DoNotLock")
    (UserInterface|Viewport|AddtoViewport (Variables|Default|GetpauseMenu) 0)
    (Game|SetGamePaused true)))

(fn ConstructionScript
  (Transformation|AttachComponentToComponent (Variables|Default|GetcarWeapon) (Variables|Character|GetMesh) "turret" "SnapToTarget" "SnapToTarget" "SnapToTarget" true))