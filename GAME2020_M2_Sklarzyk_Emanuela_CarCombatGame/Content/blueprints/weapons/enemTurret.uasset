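; Enemy turret that tracks and shoots at player 0's pawn while it is within attack range.
; Each Tick updates the range flag, then drives rotation and firing from it.
; The top eases toward the player using RInterpTo, with pitch offset by BarrelLength and clamped.
; A Delay called from Tick paces fire, spawning projectiles at the spawnPoint socket without rechecking range afterward.
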(event Custom|updateRotation
  (bind _returnvalue (Game|Player|GetPlayerPawn 0))
  (bind _turrtop (Variables|Default|GetturrTop))
  (bind _returnvalue_2 (Transformation|GetActorLocation _returnvalue))
  (bind _returnvalue_3 (Transformation|GetWorldLocation _turrtop))
  (bind _returnvalue_4 (Math|Rotator|FindLookatRotation _returnvalue_3 _returnvalue_2))
  (bind (_roll _pitch _yaw) (Math|Rotator|BreakRotator _returnvalue_4))
  ;[1 1 1] turretRotation
  (if (Variables|Default|GetenemInRange)
    (Transformation|SetWorldRotation (Variables|Default|GetturrTop) (Math|Interpolation|RInterpTo (Transformation|GetWorldRotation (Variables|Default|GetturrTop)) (Math|Rotator|MakeRotator 0.0 (Math|Float|ClampAngle (- _pitch (Variables|TurretSettings|GetbarrelLength)) -1e+01 4e+01) _yaw) (Variables|Default|GetdeltaTime) (Variables|TurretSettings|GetrotSpeed)) false false)))

(event Custom|fireWeapons
  ;[1 1 1] fireWeapons
  (if (Variables|Default|GetenemInRange)
    (Utilities|FlowControl|Delay (Variables|TurretSettings|GetfireInterval))
    (Game|SpawnActorfromClass "/Game/blueprints/weapons/projectile.projectile_C" (Transformation|GetSocketTransform (Variables|Default|GetturrTop) "spawnPoint" "RTS_World") "Undefined" 0 0)))

(event Custom|updateRange
  ;[1 1 1] updates
  (if (<= (Transformation|GetDistanceTo self (Game|Player|GetPlayerPawn 0)) (Variables|TurretSettings|GetattackRange))
    (Variables|Default|SetenemInRange true)
    (else
      (Variables|Default|SetenemInRange false))))

(event EventTick
  (params (DeltaSeconds :type Float%20%28single-precision%29))
  ;[1 1 1] updates
  (Variables|Default|SetdeltaTime DeltaSeconds)
  (CallFunction|UpdateRange)
  (CallFunction|UpdateRotation)
  (CallFunction|FireWeapons))

(fn ConstructionScript)