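; Enemy turret hazard that turns toward a Character inside its Range component.
; Overlap begin stores the Character and opens a Tick gate; overlap end closes it.
; While open, each tick interpolates TurPoint toward the Character's mesh using RInterpTo with a fixed delta time, then calls SpawnProjectile.
; SpawnProjectile does nothing as wired: its timed fire-delay and projectile-spawning logic is disconnected.
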(event OnComponentBeginOverlap(range)
  (params (OverlappedComponent :type Primitive%20Component%20Object%20Reference) (OtherActor :type Actor%20Object%20Reference) (OtherComp :type Primitive%20Component%20Object%20Reference) (OtherBodyIndex :type Integer) (bFromSweep :type Boolean) (SweepResult :type Hit%20Result%20Structure%20%28by%20ref%29))
  (bind _rottop (Variables|Default|GetrotTop))
  (bind _ascharacter (Utilities|Casting|CastToCharacter OtherActor))
  (Utilities|FlowControl|Gate true) ; enters at Open
)

(event OnComponentEndOverlap(range)
  (params (OverlappedComponent :type Primitive%20Component%20Object%20Reference) (OtherActor :type Actor%20Object%20Reference) (OtherComp :type Primitive%20Component%20Object%20Reference) (OtherBodyIndex :type Integer))
  (bind _rottop (Variables|Default|GetrotTop))
  (Utilities|Casting|CastToCharacter OtherActor)
  (Utilities|FlowControl|Gate true) ; enters at Close
)

(event EventTick
  (params (DeltaSeconds :type Float%20%28single-precision%29))
  (bind _rottop (Variables|Default|GetrotTop))
  (Utilities|FlowControl|Gate true
    (:Exit
      (Transformation|SetWorldRotation (Variables|Default|GetturPoint) (Math|Interpolation|RInterpTo (Transformation|GetWorldRotation _rottop) (Math|Rotator|FindLookatRotation (Transformation|GetWorldLocation _rottop) (Transformation|GetWorldLocation (Variables|/Script/Engine.Character|GetMesh (stale OnComponentBeginOverlap(range) _ascharacter)))) 2.0 (Variables|Default|GetrotSpeed)) false false)
      (CallFunction|SpawnProjectile))))

(fn ConstructionScript)

(fn SpawnProjectile)